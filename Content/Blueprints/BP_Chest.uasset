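; Treasure chest actor that opens when the player enters its trigger box and throws out a health pickup.
; Box overlap with the cached player character plays a timeline that drives the lid's roll rotation.
; When the timeline finishes, it spawns BP_HealthPickUp at the Scene transform, enables physics and launches it with an impulse.
; There is no one-shot guard, so re-entering replays the opening from the start.
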(event `self.ReceiveBeginPlay`
  ;[1 0.48 0.683] Get Player Ref
  (bind _asbp_third_person_character (cast `/Game/ThirdPerson/Blueprints/BP_ThirdPersonCharacter` (`GameplayStatics.GetPlayerCharacter` 0)))
  (set `self.PlayerRef` _asbp_third_person_character))

(event `self.Box.OnComponentBeginOverlap`
  (params (OverlappedComponent :type "PrimitiveComponent Object Reference") (OtherActor :type "Actor Object Reference") (OtherComp :type "PrimitiveComponent Object Reference") (OtherBodyIndex :type Integer) (bFromSweep :type Boolean) (SweepResult :type "HitResult Structure (by ref)"))
  (bind _lid (`self.lid`))
  (bind (_relativerotation_roll _relativerotation_pitch _relativerotation_yaw) (`KismetMathLibrary.BreakRotator` (`SceneComponent.RelativeRotation` _lid)))
  ;[0.6979 1 0.37] Chest Open
  (if (== OtherActor (`self.PlayerRef`))
    (bind (_direction _rotate) (`Timeline|Open_led` :!via `PlayFromStart`)
      (:`Update`
        (`SceneComponent.K2_SetRelativeRotation` _lid (`KismetMathLibrary.MakeRotator` (* _rotate -1.0) _relativerotation_pitch _relativerotation_yaw) false false))
      (:`Finished`
        (`self.SpawnItem`)))))

(event `self.Box.OnComponentEndOverlap`
  (params (OverlappedComponent :type "PrimitiveComponent Object Reference") (OtherActor :type "Actor Object Reference") (OtherComp :type "PrimitiveComponent Object Reference") (OtherBodyIndex :type Integer))
  ;[0.6979 1 0.37] Chest Open
  (if (== OtherActor (`self.PlayerRef`))
    _))

(event `SpawnItem`
  ;[1 1 1] Spawn
  (bind _returnvalue (`|SpawnActorFromClass` "/Game/Blueprints/BP_HealthPickUp.BP_HealthPickUp_C" (`SceneComponent.K2_GetComponentToWorld` (`self.Scene`)) "Undefined" "MultiplyWithRoot" null null))
  (bind _staticmesh (`/Game/Blueprints/BP_HealthPickUp.StaticMesh` _returnvalue))
  (`PrimitiveComponent.SetSimulatePhysics` _staticmesh true)
  (`PrimitiveComponent.AddImpulseAtLocation` _staticmesh (0.0 1000.0 5000.0) (`self.K2_GetActorLocation` _returnvalue) "None"))

(fn `UserConstructionScript`)