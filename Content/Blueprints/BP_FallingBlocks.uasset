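; BP_FallingBlocks is a block that starts to fall when the player character overlaps its Box trigger.
; BeginPlay caches the player as BP_ThirdPersonCharacter, and the overlap plays the Fall timeline only for that actor.
; Each timeline update adds Alpha times MoveBy to the static mesh's current world Z, so the offset accumulates per tick rather than interpolating from a stored start position.
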(event `self.ReceiveBeginPlay`
  ;[1 0.17 0.7499] playere reference
  (bind _asbp_third_person_character (cast `/Game/ThirdPerson/Blueprints/BP_ThirdPersonCharacter` (`GameplayStatics.GetPlayerCharacter` 0)))
  (set `self.player ref` _asbp_third_person_character))

(event `self.Box.OnComponentBeginOverlap`
  (params (OverlappedComponent :type "PrimitiveComponent Object Reference") (OtherActor :type "Actor Object Reference") (OtherComp :type "PrimitiveComponent Object Reference") (OtherBodyIndex :type Integer) (bFromSweep :type Boolean) (SweepResult :type "HitResult Structure (by ref)"))
  (bind _staticmesh (`self.StaticMesh`))
  (if (== OtherActor (`self.player ref`))
    (bind (_direction _alpha) (`Timeline|fall`)
      (:`Update`
        (bind (_returnvalue_x _returnvalue_y _returnvalue_z) (`KismetMathLibrary.BreakVector` (+ (`SceneComponent.K2_GetComponentLocation` _staticmesh) (`KismetMathLibrary.MakeVector` 0.0 0.0 (* _alpha (`self.moveBy`))))))
        (`SceneComponent.K2_SetWorldLocation` _staticmesh (`KismetMathLibrary.MakeVector` _returnvalue_x _returnvalue_y _returnvalue_z) false false)))))

(fn `UserConstructionScript`)