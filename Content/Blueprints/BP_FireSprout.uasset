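; BP_FireSprout is a fire trap that burns the player while they stand inside its box.
; Box overlap events show and hide the fire particle system after short delays when the player enters or leaves.
; Tick applies damage while the fire is visible and overlaps the cached player, using a DoOnce reset by a Delay as a once-per-second cooldown.
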(event `self.ReceiveBeginPlay`
  ;[0.53 0 0.1198] Player Reference
  (bind _asbp_third_person_character (cast `/Game/ThirdPerson/Blueprints/BP_ThirdPersonCharacter` (`GameplayStatics.GetPlayerCharacter` 0)))
  (set `self.Player Ref` _asbp_third_person_character))

(event `self.ReceiveTick`
  (params (DeltaSeconds :type "Float (single-precision)"))
  (bind _player_ref (`self.Player Ref`))
  ;[0.75 0 0.3236] Damage System
  (if (`SceneComponent.IsVisible` (`self.ParticleSystem`))
    (if (`PrimitiveComponent.IsOverlappingActor` (`self.Box`) _player_ref)
      (`/Engine/EditorBlueprintResources/StandardMacros.DoOnce` false :!label _label
        (:`Completed`
          (`GameplayStatics.ApplyDamage` _player_ref 10.0)
          (`KismetSystemLibrary.Delay` 1.0)
          (goto _label :!via `Reset`))))))

(event `self.Box.OnComponentBeginOverlap`
  (params (OverlappedComponent :type "PrimitiveComponent Object Reference") (OtherActor :type "Actor Object Reference") (OtherComp :type "PrimitiveComponent Object Reference") (OtherBodyIndex :type Integer) (bFromSweep :type Boolean) (SweepResult :type "HitResult Structure (by ref)"))
  ;[1 0.9737 0.52] Fire
  (if (== OtherActor (`self.Player Ref`))
    (`KismetSystemLibrary.Delay` 0.2)
    (`SceneComponent.SetVisibility` (`self.ParticleSystem`) true false)))

(event `self.Box.OnComponentEndOverlap`
  (params (OverlappedComponent :type "PrimitiveComponent Object Reference") (OtherActor :type "Actor Object Reference") (OtherComp :type "PrimitiveComponent Object Reference") (OtherBodyIndex :type Integer))
  ;[1 0.9737 0.52] Fire
  (if (== OtherActor (`self.Player Ref`))
    (`KismetSystemLibrary.Delay` 1.0)
    (`SceneComponent.SetVisibility` (`self.ParticleSystem`) false false)))

(fn `UserConstructionScript`)