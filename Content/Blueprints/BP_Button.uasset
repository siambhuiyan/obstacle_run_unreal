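; BP_Button is a pressure button that opens and closes a linked gate as the player steps on and off it.
; A sphere overlap with the cached third-person player pawn sets IsOpen and plays or reverses the Button_press timeline.
; The timeline drives the mesh's absolute world Z, and on finishing calls GateOpen or GateClose on GateObj according to IsOpen.
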(event `self.ReceiveBeginPlay`
  ;[1 1 1] Player Ref
  (bind _asbp_third_person_character (cast `/Game/ThirdPerson/Blueprints/BP_ThirdPersonCharacter` (`GameplayStatics.GetPlayerPawn` 0)))
  (set `self.PlayerRef` _asbp_third_person_character))

(event `self.Sphere.OnComponentBeginOverlap`
  (params (OverlappedComponent :type "PrimitiveComponent Object Reference") (OtherActor :type "Actor Object Reference") (OtherComp :type "PrimitiveComponent Object Reference") (OtherBodyIndex :type Integer) (bFromSweep :type Boolean) (SweepResult :type "HitResult Structure (by ref)"))
  (bind _gate_obj (`self.gate_obj`))
  (bind (_returnvalue_x _returnvalue_y) (`KismetMathLibrary.BreakVector` (`SceneComponent.K2_GetComponentLocation` (`self.StaticMesh`))))
  ;[1 1 1] Button Press
  (if (== OtherActor (`self.PlayerRef`))
    (set `self.isOpen` true)
    (bind (_direction _z_height) (`Timeline|button_press` :!label _label)
      (:`Update`
        (`SceneComponent.K2_SetWorldLocation` (`self.StaticMesh`) (`KismetMathLibrary.MakeVector` _returnvalue_x _returnvalue_y _z_height) false false))
      (:`Finished`
        ;[1 0.9 0.27] Button Press And Open Door
        (if (`self.isOpen`)
          (`/Engine/EditorBlueprintResources/StandardMacros.IsValid` _gate_obj
            (:`Is Valid`
              (`/Game/Blueprints/BP_Gate.Gate Open` _gate_obj)))
          (else
            (`/Engine/EditorBlueprintResources/StandardMacros.IsValid` _gate_obj
              (:`Is Valid`
                (`/Game/Blueprints/BP_Gate.Gate Close` _gate_obj)))))))))

(event `self.Sphere.OnComponentEndOverlap`
  (params (OverlappedComponent :type "PrimitiveComponent Object Reference") (OtherActor :type "Actor Object Reference") (OtherComp :type "PrimitiveComponent Object Reference") (OtherBodyIndex :type Integer))
  ;[1 1 1] Button Press
  (if (== OtherActor (`self.PlayerRef`))
    (set `self.isOpen` false)
    (goto _label :!via `Reverse`)))

(fn `UserConstructionScript`)