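; BP_HealthPickUp is a pickup actor that restores the player's health when they overlap its sphere.
; On BeginPlay it casts player character 0 to BP_ThirdPersonCharacter and caches the reference.
; On sphere overlap by that player, if health is below the maximum, it adds HealAmount, clamps the result and destroys itself, so it remains in place at full health.
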(event `self.ReceiveBeginPlay`
  ;[1 1 1] Cast To Player
  (bind _asbp_third_person_character (cast `/Game/ThirdPerson/Blueprints/BP_ThirdPersonCharacter` (`GameplayStatics.GetPlayerCharacter` 0)))
  (set `self.PlayreRef` _asbp_third_person_character))

(event `self.Sphere.OnComponentBeginOverlap`
  (params (OverlappedComponent :type "PrimitiveComponent Object Reference") (OtherActor :type "Actor Object Reference") (OtherComp :type "PrimitiveComponent Object Reference") (OtherBodyIndex :type Integer) (bFromSweep :type Boolean) (SweepResult :type "HitResult Structure (by ref)"))
  (bind _currenthelath (`/Game/ThirdPerson/Blueprints/BP_ThirdPersonCharacter.currentHelath` (`self.PlayreRef`)))
  ;[0.01 1 0.08459] Health Pickup
  (if (== OtherActor (`self.PlayreRef`))
    (if (< _currenthelath 100.0)
      (set `/Game/ThirdPerson/Blueprints/BP_ThirdPersonCharacter.currentHelath` (`KismetMathLibrary.FClamp` (+ _currenthelath (`self.healAmount`)) 0.0 100.0) (`self.PlayreRef`))
      (`self.K2_DestroyActor`))))

(fn `UserConstructionScript`)