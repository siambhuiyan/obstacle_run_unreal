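; BP_Door is a door actor that swings open when the third-person character enters its box trigger and reverses when that character leaves.
; The overlap events play and reverse the DoorOpen timeline, whose scaled Alpha track sets the Door component's relative yaw.
; An event track on the same timeline checks playback direction to play a different sound at the door for opening and closing.
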(event `self.Box.OnComponentBeginOverlap`
  (params (OverlappedComponent :type "PrimitiveComponent Object Reference") (OtherActor :type "Actor Object Reference") (OtherComp :type "PrimitiveComponent Object Reference") (OtherBodyIndex :type Integer) (bFromSweep :type Boolean) (SweepResult :type "HitResult Structure (by ref)"))
  (bind _returnvalue (`SceneComponent.K2_GetComponentLocation` (`self.door`)))
  (cast `/Game/ThirdPerson/Blueprints/BP_ThirdPersonCharacter` OtherActor)
  (bind (_direction _alpha) (`Timeline|door open` :!label _label)
    (:`Update`
      (`SceneComponent.K2_SetRelativeRotation` (`self.door`) (`KismetMathLibrary.MakeRotator` 0.0 0.0 (* _alpha 1000.0)) false false))
    (:`open sound`
      (switch `ETimelineDirection` _direction
        (:`Forward`
          (`GameplayStatics.PlaySoundAtLocation` "/Game/StarterContent/Audio/Collapse01.Collapse01" _returnvalue (struct) 1.0 1.0 0.0 null null null null))
        (:`Backward`
          (`GameplayStatics.PlaySoundAtLocation` "/Game/StarterContent/Audio/Collapse02.Collapse02" _returnvalue (struct) 1.0 1.0 0.0 null null null null))))))

(event `self.Box.OnComponentEndOverlap`
  (params (OverlappedComponent :type "PrimitiveComponent Object Reference") (OtherActor :type "Actor Object Reference") (OtherComp :type "PrimitiveComponent Object Reference") (OtherBodyIndex :type Integer))
  (cast `/Game/ThirdPerson/Blueprints/BP_ThirdPersonCharacter` OtherActor)
  (goto _label :!via `Reverse`))

(fn `UserConstructionScript`)